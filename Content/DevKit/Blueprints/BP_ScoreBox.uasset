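; Shootable score target that registers with BP_FirstPersonGameMode on BeginPlay and awards points when destroyed.
; Any damage lowers its health and replays a timeline-driven colour flash on a dynamic material instance, with the play rate scaled from the flash duration.
; At zero health it breaks once, spawning an effect and sound, reporting points to the game mode and destroying itself.
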(event Custom|PlayHitFlash
  (bind _fade (Timeline|HitFlash PlayFromStart)
    (:Update
      (Rendering|Material|SetScalarParameterValue (Variables|HitSettings|GetHitMID) (Variables|HitSettings|GetHitAmountParam) _fade :!class /Script/Engine.MaterialInstanceDynamic))))

(event EventBeginPlay
  (bind _asbp_first_person_game_mode (Utilities|Casting|CastToBP_FirstPersonGameMode (Game|GetGameMode)))
  (bind _output_get (Variables|Default|SetGameModeRef _asbp_first_person_game_mode))
  (Default|RegisterTarget _output_get)
  (bind _returnvalue (Rendering|Material|CreateDynamicMaterialInstance (Variables|Default|GetStaticMesh) 0 0 "None" :!class /Script/Engine.PrimitiveComponent))
  (bind _output_get_2 (Variables|HitSettings|SetHitMID _returnvalue))
  (Rendering|Material|SetVectorParameterValue _output_get_2 (Variables|HitSettings|GetHitColourParam) (Variables|HitSettings|GetHitColour) :!class /Script/Engine.MaterialInstanceDynamic)
  (Components|Timeline|SetPlayRate (Variables|Default|GetHitFlash) (Math|Float|SafeDivide 1.0 (Variables|HitSettings|GetHitFlashDuration))))

(event Game|Damage|EventAnyDamage
  (params (Damage :type Float%20%28single-precision%29) (DamageType :type Damage%20Type%20Object%20Reference) (InstigatedBy :type Controller%20Object%20Reference) (DamageCauser :type Actor%20Object%20Reference))
  (bind _returnvalue (Transformation|GetActorLocation))
  (if (not (Variables|BoxSettings|GetbBroken))
    (bind _output_get (Variables|BoxSettings|SetBoxHealth (- (Variables|BoxSettings|GetBoxHealth) Damage)))
    (CallFunction|PlayHitFlash)
    (if (<= _output_get 0.0)
      (Variables|BoxSettings|SetbBroken true)
      (Effects|SpawnEmitteratLocation (Variables|BoxSettings|GetBreakFX) _returnvalue)
      (Audio|PlaySoundatLocation (Variables|BoxSettings|GetBreakSound) _returnvalue "0, 0, 0" 1.0 1.0 0.0 0 0 0 0)
      (Default|TargetDestroyed (Variables|Default|GetGameModeRef) (Variables|BoxSettings|GetPointsPerBox))
      (Actor|DestroyActor))))

(fn ConstructionScript)