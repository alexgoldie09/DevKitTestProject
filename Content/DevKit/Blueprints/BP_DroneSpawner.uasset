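; Spawner actor that periodically populates a box area with drones up to a live-count cap.
; On BeginPlay it async-loads the drone class, then starts a looping timer that spawns at random points within the SpawnArea box.
; Spawns skip colliding spots, and each drone's OnDestroyed event decrements the alive count so replacements can follow.
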(event Custom|TrySpawn
  (bind _spawnarea (Variables|Default|GetSpawnArea))
  (if (< (Variables|Default|GetAliveCount) (Variables|Default|GetMaxAlive))
    (bind _returnvalue (Game|SpawnActorfromClass (Variables|Default|GetLoadedDroneClass) (Math|Transform|MakeTransform (Math|Random|RandomPointinBoundingBox (Transformation|GetWorldLocation _spawnarea) (Components|Box|GetScaledBoxExtent _spawnarea))) "AdjustIfPossibleButDontSpawnIfColliding" "MultiplyWithRoot" 0 0))
    (Utilities|IsValid _returnvalue
      (:Is%20Valid
        (Math|Integer|IncrementInt (Variables|Default|GetAliveCount)
          (:%20%20
            (Game|BindEventtoOnDestroyed _returnvalue (delegate Custom|DroneGone))))))))

(event Custom|DroneGone
  (params (DestroyedActor :type Actor%20Object%20Reference))
  (Variables|Default|SetAliveCount (Math|Integer|Max(Integer) (- (Variables|Default|GetAliveCount) 1))))

(event EventBeginPlay
  (bind _class (Utilities|AsyncLoadClassAsset (Variables|Default|GetDroneClass))
    (:Completed
      (bind _asactor (Utilities|Casting|CastToActorClass _class))
      (Variables|Default|SetLoadedDroneClass _asactor)
      (Utilities|Time|SetTimerbyEvent (delegate Custom|TrySpawn) (Variables|Default|GetSpawnInterval) true false (Variables|Default|GetFirstSpawnDelay)))))

(fn ConstructionScript)