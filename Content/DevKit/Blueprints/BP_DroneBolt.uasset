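; BP_DroneBolt is a projectile, apparently fired by a drone, that damages the player pawn on impact.
; On begin play its collision sphere ignores the owning actor during movement, and its mesh gets a dynamic material tinted by GlowColour.
; On any hit it destroys itself, first applying BoltDamage if the other actor is the player pawn.
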(event EventBeginPlay
  (Collision|IgnoreActorwhenMoving (Variables|Default|GetSphere) (Components|GetOwner) true)
  (bind _returnvalue (Rendering|Material|CreateDynamicMaterialInstance (Variables|Default|GetMesh) 0 0 "None" :!class /Script/Engine.PrimitiveComponent))
  (Rendering|Material|SetVectorParameterValue _returnvalue "GlowColour" (Variables|Default|GetGlowColour) :!class /Script/Engine.MaterialInstanceDynamic))

(event Collision|EventHit
  (params (MyComp :type Primitive%20Component%20Object%20Reference) (Other :type Actor%20Object%20Reference) (OtherComp :type Primitive%20Component%20Object%20Reference) (bSelfMoved :type Boolean) (HitLocation :type Vector :default "0, 0, 0") (HitNormal :type Vector :default "0, 0, 0") (NormalImpulse :type Vector :default "0, 0, 0") (Hit :type Hit%20Result%20Structure%20%28by%20ref%29))
  (if (== Other (Game|Player|GetPlayerPawn 0))
    (Game|Damage|ApplyDamage Other (Variables|Default|GetBoltDamage) 0 self)
    (Actor|DestroyActor)
    (else
      (Actor|DestroyActor))))

(fn ConstructionScript)